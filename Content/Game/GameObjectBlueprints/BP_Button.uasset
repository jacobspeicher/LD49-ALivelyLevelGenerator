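; BP_Button is a damage-activated button that slides a pair of referenced door actors apart.
; Any damage calls MoveDoors, which, while the button is usable, starts opening and turns a button material blue.
; Tick moves the doors in opposite directions along Direction at Speed, drawing the left door's location as debug text.
; Once that door's world X drops below LeftDoorOpen, movement stops and the button becomes unusable.
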(event EventBeginPlay)

(event Collision|EventActorBeginOverlap
  (params (OtherActor :type Actor%20Object%20Reference)))

(event EventTick
  (params (DeltaSeconds :type Float%20%28single-precision%29))
  (bind _returnvalue (Utilities|Time|GetWorldDeltaSeconds))
  (bind _leftdoor (Variables|Default|GetLeftDoor))
  (bind _rightdoor (Variables|Default|GetRightDoor))
  (bind _direction (Variables|Default|GetDirection))
  (bind _speed (Variables|Default|GetSpeed))
  (bind _leftdoor_2 (Variables|Default|GetLeftDoor))
  (bind _returnvalue_2 (Transformation|GetActorTransform _rightdoor))
  (bind _returnvalue_3 (Transformation|GetActorLocation _leftdoor_2))
  (bind _returnvalue_4 (Math|Vector|Normalize _direction))
  (bind _returnvalue_5 (Transformation|GetActorTransform _leftdoor))
  (bind _returnvalue_6 (* _returnvalue _speed))
  (bind (_location _rotation _scale) (Math|Transform|BreakTransform _returnvalue_2))
  (bind _returnvalue_7 (* _returnvalue_4 _returnvalue_6))
  (bind (_location_2 _rotation_2 _scale_2) (Math|Transform|BreakTransform _returnvalue_5))
  (if (Variables|Default|GetOpen)
    (Transformation|SetActorTransform (Variables|Default|GetLeftDoor) (Math|Transform|MakeTransform (+ (* _returnvalue_7 -1.0) _location_2) _rotation_2 _scale_2))
    (Transformation|SetActorTransform (Variables|Default|GetRightDoor) (Math|Transform|MakeTransform (+ _returnvalue_7 _location) _rotation _scale))
    (Rendering|Debug|DrawDebugString _returnvalue_3 (Utilities|String|ToString(Vector) _returnvalue_3) 0 "(R=1.000000,G=0.000000,B=0.000000,A=1.000000)")
    (if (< (.X (Math|Vector|BreakVector _returnvalue_3)) (Variables|Default|GetLeftDoorOpen))
      (Variables|Default|SetOpen false)
      (Variables|Default|SetUsable false))))

(event Game|Damage|EventAnyDamage
  (params (Damage :type Float%20%28single-precision%29) (DamageType :type Damage%20Type%20Object%20Reference) (InstigatedBy :type Controller%20Object%20Reference) (DamageCauser :type Actor%20Object%20Reference))
  (CallFunction|MoveDoors))

(fn ConstructionScript)

(fn MoveDoors
  (if (Variables|Default|GetUsable)
    (Variables|Default|SetOpen true)
    (Rendering|Material|SetMaterial (Variables|Default|GetButton) 1 "/Game/Materials/Blue.Blue")))